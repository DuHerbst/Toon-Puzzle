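; BP_PhysicsCube is an interactable cube the player can pick up and drop, with a toggleable prompt and a configurable material.
; Interact toggles between OnPickup and OnDrop based on IsCarried.
; Pickup disables physics and collision, attaches the cube to BP_MyCharacter's CubeHoldPoint and updates the carrier's held state.
; Drop detaches it, restores physics, and sets its location from the carrier's forward vector plus an offset, omitting the carrier's position.
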(event EventShowPrompt
  (Rendering|SetVisibility (Variables|Default|GetToastInteract) true false))

(event EventHidePrompt
  (Rendering|SetVisibility (Variables|Default|GetToastInteract) false false))

(event EventInteract
  (bind _asbp_my_character (Utilities|Casting|CastToBP_MyCharacter (Game|GetPlayerCharacter 0)))
  (Variables|Default|SetCarrier _asbp_my_character)
  (if (Variables|Default|GetIsCarried?)
    (CallFunction|OnDrop)
    (else
      (CallFunction|OnPickup))))

(fn ConstructionScript
  (Rendering|Material|SetMaterial (Variables|Default|GetPhysicsCube) 0 (Variables|Default|GetMaterialChange)))

(fn OnPickup
  (bind _carrier (Variables|Default|GetCarrier))
  (Physics|SetSimulatePhysics (Variables|Default|GetPhysicsCube) false)
  (Physics|SetEnableGravity (Variables|Default|GetPhysicsCube) false)
  (Variables|Default|SetIsCarried? true)
  (Collision|SetCollisionEnabled (Variables|Default|GetPhysicsCube) "NoCollision")
  (Transformation|AttachComponentToComponent (Variables|Default|GetPhysicsCube) (Variables|/Game/DHA_Assignment2/Blueprints/BP_MyCharacter.BP_MyCharacter_C|GetCubeHoldPoint (Variables|Default|GetCarrier)) "None" "SnapToTarget" "SnapToTarget" "KeepRelative" true)
  (Variables|/Game/DHA_Assignment2/Blueprints/BP_MyCharacter.BP_MyCharacter_C|SetHeldCube _carrier self)
  (Variables|/Game/DHA_Assignment2/Blueprints/BP_MyCharacter.BP_MyCharacter_C|SetIsHoldingCube? _carrier true))

(fn OnDrop
  (Development|PrintString "Thing dropped")
  (Transformation|DetachFromActor "KeepRelative" "KeepRelative" "KeepRelative")
  (Transformation|SetActorLocation (+ (* (Transformation|GetActorForwardVector (Variables|Default|GetCarrier)) 100) "50.000000,50.000000,50.000000") false false)
  (Collision|SetCollisionEnabled (Variables|Default|GetPhysicsCube) "QueryAndPhysics")
  (Physics|SetSimulatePhysics (Variables|Default|GetPhysicsCube) true)
  (Physics|SetEnableGravity (Variables|Default|GetPhysicsCube) true)
  (Variables|Default|SetIsCarried? false)
  (Variables|Default|SetHeld%20Cube self)
  (Variables|/Game/DHA_Assignment2/Blueprints/BP_MyCharacter.BP_MyCharacter_C|SetIsHoldingCube? (Variables|Default|GetCarrier) false))