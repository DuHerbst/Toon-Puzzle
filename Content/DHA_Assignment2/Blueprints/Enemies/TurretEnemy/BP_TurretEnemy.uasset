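; Turret enemy that sweeps back and forth in yaw around its starting rotation and can fire shoot cubes.
; While scanning is on, Tick calls ScanForPlayer, which moves a frame-rate-independent offset between the angle limits and reverses at each end; it performs no player detection.
; A separate Shoot event, not called within this Blueprint, spawns a BP_ShootCube at the muzzle, followed by a delay that leads nowhere.
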(event Custom|Shoot
  (Game|SpawnActorfromClass "/Game/DHA_Assignment2/Blueprints/BP_ShootCube.BP_ShootCube_C" (Math|Transform|MakeTransform (Transformation|GetWorldLocation (Variables|Default|GetMuzzleShot)) (Transformation|GetWorldRotation (Variables|Default|GetMuzzleShot))) "Undefined" "MultiplyWithRoot" 0 0)
  (Utilities|FlowControl|Delay 1.0))

(event EventBeginPlay
  (Variables|Default|SetStartRotation (Transformation|GetActorRotation)))

(event EventTick
  (params (DeltaSeconds :type Float%20%28single-precision%29))
  (if (Variables|Default|GetIsScanning)
    (CallFunction|ScanforPlayer)))

(fn ConstructionScript)

(fn ScanforPlayer
  (Variables|Default|SetCurrentOffset (Math|Float|Clamp(Float) (+ (Variables|Default|GetCurrentOffset) (* (Variables|Default|GetScanSpeed) (Variables|Default|GetScanDirection) (Utilities|Time|GetWorldDeltaSeconds))) (* (Variables|Default|GetScanAngle) -1.0) (Variables|Default|GetScanAngle)))
  (if (>= (Variables|Default|GetCurrentOffset) (Variables|Default|GetScanAngle))
    (Variables|Default|SetScanDirection -1.0)
    (elif (<= (Variables|Default|GetCurrentOffset) (* (Variables|Default|GetScanAngle) -1.0))
      (Variables|Default|SetScanDirection 1.0)
      (else
        (Transformation|SetActorRotation (Math|Rotator|MakeRotator 0.0 0.0 (+ (.Yaw (Math|Rotator|BreakRotator (Variables|Default|GetStartRotation))) (Variables|Default|GetCurrentOffset))))))))