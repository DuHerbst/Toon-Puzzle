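; BP_Keys is a spinning, collectible key pickup whose KeyMesh is configured per KeyType by SetKey and KeyMap in the construction script.
; It shows or hides an interaction prompt on request.
; Interact plays Niagara and sound effects, passes the key to BP_MyCharacter and, after a short delay, its HUD, then destroys the actor.
; Switchon sets Activated and slides the mesh toward EndLocationKey with a Timeline-driven lerp.
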(event EventBeginPlay
  (Variables|Default|SetStart%20LocationKey (Variables|/Script/Engine.SceneComponent|GetRelativeLocation (Variables|Default|GetKeyMesh)))
  (Variables|Default|SetActivated? false))

(event EventShowPrompt
  (Rendering|SetVisibility (Variables|Default|GetInteractionToast) true false))

(event EventHidePrompt
  (Rendering|SetVisibility (Variables|Default|GetInteractionToast) false false))

(event EventSwitchon
  (Variables|Default|SetActivated? true)
  (bind _movementalpha (Timeline|Timeline Play)
    (:Update
      (Transformation|SetRelativeLocation (Variables|Default|GetKeyMesh) (Math|Vector|Lerp(Vector) (Variables|Default|GetStart%20LocationKey) (Variables|Default|GetEnd%20LocationKey) _movementalpha) false false))))

(event EventInteract
  (bind _asbp_my_character (Utilities|Casting|CastToBP_MyCharacter (Game|GetPlayerCharacter 0)))
  (AddComponent|AddNiagaraComponent false)
  (Audio|PlaySound2D "/Game/DHA_Assignment2/SFXAudio/PickupKey.PickupKey" 1.0 1.0 0.0 0 0)
  (Class|BPIPlayerKeys|AddKey(Message) _asbp_my_character (Variables|Setup|GetKeyType))
  (Utilities|FlowControl|Delay 0.2)
  (Default|AddKeyHUD (Variables|/Game/DHA_Assignment2/Blueprints/BP_MyCharacter.BP_MyCharacter_C|GetPlayerHUD _asbp_my_character) (Variables|Default|GetKeyTypes))
  (Actor|DestroyActor))

(event EventTick
  (params (DeltaSeconds :type Float%20%28single-precision%29))
  (Transformation|AddActorLocalRotation (Math|Rotator|MakeRotator 0.0 0.0 (* DeltaSeconds (Variables|Default|GetRotation))) false false))

(fn ConstructionScript
  (CallFunction|SetKey (Utilities|Array|MakeArray (Variables|Default|GetKeyMesh)) (Variables|Default|GetKeyMap) (Variables|Setup|GetKeyType)))