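; BP_Switch is a pressure-plate style switch that responds to a BP_PhysicsCube whose type matches its required cube type.
; A matching overlap sets the on material, plays a plate sound and sends SwitchOnMessage to each linked interact element.
; For one particular required type, that loop also calls CheckWin on the win-check reference.
; When no overlapping actors of any kind remain, it restores the off material and sends SwitchOffMessage to those elements.
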(event OnComponentBeginOverlap(Collider)
  (params (OverlappedComponent :type Primitive%20Component%20Object%20Reference) (OtherActor :type Actor%20Object%20Reference) (OtherComp :type Primitive%20Component%20Object%20Reference) (OtherBodyIndex :type Integer) (bFromSweep :type Boolean) (SweepResult :type Hit%20Result%20Structure%20%28by%20ref%29))
  (bind _asbp_physics_cube (Utilities|Casting|CastToBP_PhysicsCube OtherActor))
  (if (Utilities|Enum|Equal(Enum) (Variables|/Game/DHA_Assignment2/Blueprints/BP_PhysicsCube.BP_PhysicsCube_C|GetCubeType _asbp_physics_cube) (Variables|Setup|GetRequiredCubeType))
    (CallFunction|Experience)
    (for _array_element (Variables|Setup|GetInteractElements)
      (Class|BPIInteract|Switchon(Message) _array_element)
      (if (Utilities|Enum|Equal(Enum) (Variables|Setup|GetRequiredCubeType) "NewEnumerator2")
        (Default|CheckWin (Variables|WinConditions|GetWinCheckRef))))))

(event OnComponentEndOverlap(Collider)
  (params (OverlappedComponent :type Primitive%20Component%20Object%20Reference) (OtherActor :type Actor%20Object%20Reference) (OtherComp :type Primitive%20Component%20Object%20Reference) (OtherBodyIndex :type Integer))
  (if (Utilities|Array|IsEmpty (Collision|GetOverlappingActors (Variables|Default|GetCollider) 0 :!class /Script/Engine.PrimitiveComponent))
    (Rendering|Material|SetMaterial (Variables|Default|GetSwitchMesh) 0 (Variables|Setup|GetSwitchOff))
    (for _array_element (Variables|Setup|GetInteractElements)
      (Class|BPIInteract|SwitchOff(Message) _array_element))))

(fn ConstructionScript
  (Rendering|Material|SetMaterial (Variables|Default|GetSwitchMesh) 0 (Variables|Setup|GetSwitchOff)))

(fn Experience
  (Rendering|Material|SetMaterial (Variables|Default|GetSwitchMesh) 0 (Variables|Setup|GetSwitchOn))
  (Audio|PlaySound2D "/Game/DHA_Assignment2/SFXAudio/PlateSound.PlateSound" 4.0 3.0 0.0 0 0))