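; BP_SwitchPlatforms is a platform actor that moves from its start position to a target position when switched on.
; On BeginPlay it stores the platform mesh's relative location and marks itself inactive.
; The Switchon event sets it active and plays a timeline that lerps the mesh between StartLocation and EndLocation without sweeping.
; The construction script applies a configurable material instance to the platform mesh.
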(event EventBeginPlay
  (Variables|Default|SetStartLocation (Variables|/Script/Engine.SceneComponent|GetRelativeLocation (Variables|Default|GetPlatformMesh)))
  (Variables|Setup|SetIsActive? false))

(event EventSwitchon
  (Variables|Setup|SetIsActive? true)
  (bind _movementalpha (Timeline|Movement%20Timeline Play)
    (:Update
      (Transformation|SetRelativeLocation (Variables|Default|GetPlatformMesh) (Math|Vector|Lerp(Vector) (Variables|Default|GetStartLocation) (Variables|Default|GetEndLocation) _movementalpha) false false))))

(fn ConstructionScript
  (Rendering|Material|SetMaterial (Variables|Default|GetPlatformMesh) 0 (Variables|Default|GetMaterialInstancePlat)))