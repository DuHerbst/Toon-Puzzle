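; BPC_Health is a health component Blueprint that holds a Health value with functions for damage and healing.
; TakeDamage subtracts the incoming damage without clamping, and its check for zero or below triggers nothing.
; HealPlayer clamps Health between 0 and 100 but adds zero, so it restores nothing as written.
; The event graph contains only disabled placeholder events.
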(event EventBeginPlay)

(event EventTick
  (params (DeltaSeconds :type Float%20%28single-precision%29)))

(fn TakeDamage
  (params (DamageTaken :type Float%20%28double-precision%29))
  (Variables|Default|SetHealth (- (Variables|Default|GetHealth) DamageTaken))
  (if (<= (Variables|Default|GetHealth) 0.0)
    _))

(fn HealPlayer
  (Variables|Default|SetHealth (Math|Float|Clamp(Float) (+ (Variables|Default|GetHealth) 0.0) 0.0 1e+02)))